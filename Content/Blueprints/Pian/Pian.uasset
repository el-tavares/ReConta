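; Interactive piano of thirteen skeletal mesh keys, each paired by position with a note widget showing an operation result from the pawn.
; Hovering highlights a key; clicking reads its note number from the component tag, broadcasts it and plays that note's sound.
; The HUD's note check tints the last clicked key green or red for right or wrong.
; The pawn's operations update refreshes the widget numbers.
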(event Custom|OnNotePlayed
  (params (RightNote :type Boolean))
  (Rendering|Material|SetOverlayMaterial (stale Custom|Clicked _asskeletal_mesh_component) (select RightNote "/Game/Art/Materials/Instances/GreenOverlay.GreenOverlay" "/Game/Art/Materials/Instances/RedOverlay.RedOverlay") :!class /Script/Engine.MeshComponent))

(event Custom|OnOperationsUpdate
  (for (_array_element _array_index) (Utilities|PianNotes)
    (bind _aspian_note (Utilities|Casting|CastToPianNote (UserInterface|GetWidget _array_element)))
    (Rendering|Components|TextRender|SetText (Variables|/Game/Blueprints/Widgets/HUD/PianNote.PianNote_C|GetNote _aspian_note) (Utilities|Text|ToText(Integer) (Utilities|Struct|BreakSOperation (.Value (Utilities|Map|Find (Variables|/Game/Blueprints/Game/RCPawn.RCPawn_C|GetOperations (Variables|Default|GetPawn)) (+ _array_index 1))))))))

(event Custom|BeginCursorOver
  (params (TouchedComponent :type Primitive%20Component%20Object%20Reference))
  (bind _asskeletal_mesh_component (Utilities|Casting|CastToSkeletalMeshComponent TouchedComponent))
  (Rendering|Material|SetOverlayMaterial _asskeletal_mesh_component "/Game/Art/Materials/Instances/WhiteOverlay.WhiteOverlay" :!class /Script/Engine.MeshComponent))

(event Custom|EndCursorOver
  (params (TouchedComponent :type Primitive%20Component%20Object%20Reference))
  (bind _asskeletal_mesh_component (Utilities|Casting|CastToSkeletalMeshComponent TouchedComponent))
  (Rendering|Material|SetOverlayMaterial _asskeletal_mesh_component 0 :!class /Script/Engine.MeshComponent))

(event Custom|Clicked
  (params (TouchedComponent :type Primitive%20Component%20Object%20Reference) (ButtonPressed :type Key%20Structure :default "None"))
  (bind _asskeletal_mesh_component (Utilities|Casting|CastToSkeletalMeshComponent TouchedComponent))
  (Default|CallOnPianPlayed (Math|Conversions|ToInteger(Byte) (Utilities|String|ToString(Name) (Utilities|Array|Get(acopy) (Variables|/Script/Engine.ActorComponent|GetComponentTags _asskeletal_mesh_component)))))
  (Audio|SpawnSound2D (Utilities|Array|Get(acopy) (Variables|Default|GetNoteSounds) (- (Math|Conversions|ToInteger(Byte) (Utilities|String|ToString(Name) (Utilities|Array|Get(acopy) (Variables|/Script/Engine.ActorComponent|GetComponentTags _asskeletal_mesh_component)))) 1)) 1.0 1.0 0.0 0))

(event EventBeginPlay
  (for _array_element (Utilities|PianKeys)
    (EventDispatchers|AssignOnBeginCursorOver _array_element (EventDispatchers|CreateEvent :!event Custom|BeginCursorOver))
    (EventDispatchers|AssignOnEndCursorOver _array_element (EventDispatchers|CreateEvent :!event Custom|EndCursorOver))
    (EventDispatchers|AssignOnClicked _array_element (EventDispatchers|CreateEvent :!event Custom|Clicked))
    (Utilities|FlowControl|DelayUntilNextTick)
    (EventDispatchers|BindEventtoOnNoteCheck (Variables|Default|GetHUD) (EventDispatchers|CreateEvent :!event Custom|OnNotePlayed))
    (EventDispatchers|BindEventtoOnOperationsUpdate (Variables|Default|GetPawn) (EventDispatchers|CreateEvent :!event Custom|OnOperationsUpdate))
    (CallFunction|OnOperationsUpdate)))

(fn ConstructionScript)