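; Player pawn that generates a set of random arithmetic operations and supplies song note data.
; UpdateOperations runs a tick after BeginPlay or on a debug key, filling an indexed map and firing an update dispatcher.
; GetValidOperation retries recursively until each operation has a positive result unique within the map.
; It also parses comma-separated song notes into integers and cycles the CineCamera's global illumination method on a key press.
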(event EventBeginPlay
  (Utilities|FlowControl|DelayUntilNextTick)
  (CallFunction|UpdateOperations))

(event Input|KeyboardEvents|DebugKeyC
  (params (Key :type Key%20Structure :default "None") (ActionValue :type Input%20Action%20Value%20Structure))
  (:Pressed
    (CallFunction|UpdateOperations)))

(event Input|KeyboardEvents|L
  (params (Key :type Key%20Structure :default "None"))
  (:Pressed
    (bind _output_get (Variables|Default|SetGlobalIllumination (select (> (Variables|Default|GetGlobalIllumination) 1) 0 (+ (Variables|Default|GetGlobalIllumination) 1))))
    (Utilities|Struct|SetmembersinPostProcessSettings (Variables|/Script/Engine.CameraComponent|GetPostProcessSettings (Variables|Default|GetCineCamera)) (Utilities|Select :Index _output_get :Option%200 "Lumen" :Option%201 "ScreenSpace" :Option%202 "None"))))

(fn ConstructionScript)

(fn GenerateRandomNumber
  (bind _output_get (LocalVariables|SetLNumber (Math|Random|RandomInteger 10)))
  (Development|PrintString (Utilities|String|ToString(Integer) _output_get) false)
  (return _output_get))

(fn GenerateRandomOperator
  (bind _output_get (LocalVariables|SetLOperator (Utilities|Select :Index (Math|Random|RandomInteger 4) :Option%200 "NewEnumerator0" :Option%201 "NewEnumerator1" :Option%202 "NewEnumerator2" :Option%203 "NewEnumerator3")))
  (Development|PrintString (Utilities|String|EnumtoString _output_get) false)
  (return _output_get))

(fn GenerateRandomOperation
  (Utilities|FlowControl|Sequence
    (:then_0
      (bind _returnvalue (CallFunction|GenerateRandomNumber))
      (LocalVariables|SetLNumber1 _returnvalue)
      (bind _returnvalue_2 (CallFunction|GenerateRandomNumber))
      (LocalVariables|SetLNumber2 _returnvalue_2)
      (bind _returnvalue_3 (CallFunction|GenerateRandomOperator))
      (LocalVariables|SetLOperator _returnvalue_3))
    (:then_1
      (switch Utilities|FlowControl|Switch|SwitchonEOperator (LocalVariables|GetLOperator)
        (:NewEnumerator0
          (LocalVariables|SetLResult (+ (LocalVariables|GetLNumber1) (LocalVariables|GetLNumber2))))
        (:NewEnumerator1
          (LocalVariables|SetLResult (- (LocalVariables|GetLNumber1) (LocalVariables|GetLNumber2))))
        (:NewEnumerator2
          (LocalVariables|SetLResult (* (LocalVariables|GetLNumber1) (LocalVariables|GetLNumber2))))
        (:NewEnumerator3
          (LocalVariables|SetLResult (/ (LocalVariables|GetLNumber1) (LocalVariables|GetLNumber2))))))
    (:then_2
      (Development|PrintString (Utilities|String|ToString(Integer) (LocalVariables|GetLResult)) false)
      (return (Utilities|Struct|MakeSOperation (LocalVariables|GetLNumber1) (LocalVariables|GetLNumber2) (LocalVariables|GetLOperator) (LocalVariables|GetLResult))))))

(fn GetValidOperation
  (params (OperationIndex :type Integer%20%28by%20ref%29))
  (bind _operation (CallFunction|GenerateRandomOperation))
  (if (> (Utilities|Struct|BreakSOperation _operation) 0)
    (bind _values (Utilities|Map|Values (Variables|Default|GetOperations)))
    (bind _array_element (Utilities|Array|ForEachLoopwithBreak _values :!label _label) ; Check if already has the result
      (:LoopBody
        (if (== (Utilities|Struct|BreakSOperation _operation) (Utilities|Struct|BreakSOperation _array_element))
          (LocalVariables|SetLHasResult true)
          (goto _label Break)
          (else
            (LocalVariables|SetLHasResult false))))
      (:Completed
        (if (LocalVariables|GetLHasResult)
          (CallFunction|GetValidOperation OperationIndex) ; Try to get diferent result
          (else
            (Utilities|Map|Add (Variables|Default|GetOperations) OperationIndex _operation)))))
    (else
      (CallFunction|GetValidOperation OperationIndex))))

(fn UpdateOperations
  (Utilities|Map|Clear (Variables|Default|GetOperations))
  (for _index (range 1 13)
    (CallFunction|GetValidOperation _index))
  (Default|CallOnOperationsUpdate))

(fn GetSongNotebyIndex
  (params (SongIndex :type Integer))
  (for _array_element (Utilities|String|ParseIntoArray (.Value (Utilities|Map|Find (Variables|/Game/Blueprints/Songs/SongData.SongData_C|GetNotes (Variables|Default|GetSongData)) SongIndex)) ",")
    (Utilities|Array|Add (LocalVariables|GetLNotes) (Math|Conversions|ToInteger(Byte) _array_element)))
  (return (LocalVariables|GetLNotes)))